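; Game mode for the menu that plays FMOD menu music and broadcasts its timeline events to other objects.
; On BeginPlay it creates an FMOD audio component with timeline callbacks enabled.
; Beats fire a beat dispatcher, plus an intensity-up dispatcher at a set bar, while markers store their name as lyrics and fire a marker dispatcher.
; A kill-music event silences the track through its Volume parameter.
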(event `self.ReceiveBeginPlay`
  (bind _returnvalue (`AddComponent|NODE_AddFMODAudioComponent-0` :`bManualAttachment` true))
  (bind _output_get (set `self.Audio Component` _returnvalue))
  (`FMODAudioComponent.SetEvent` _output_get "/Game/FMOD/Events/Music/MenuMusic.MenuMusic")
  (add `FMODAudioComponent.OnTimelineBeat` _output_get (delegate `onBeat`))
  (set `FMODAudioComponent.bEnableTimelineCallbacks` true _output_get)
  (`FMODAudioComponent.Play` _output_get)
  (add `FMODAudioComponent.OnTimelineMarker` _output_get (delegate `newMarker`)))

(event `onBeat`
  (params (Bar :type Integer) (Beat :type Integer) (Position :type Integer) (Tempo :type "Float (single-precision)") (TimeSignatureUpper :type Integer) (TimeSignatureLower :type Integer))
  (if (and (== Bar 5) (== Beat 1))
    (`self.intensityUp`))
  (`self.onBeatDisp`))

(event `newMarker`
  (params (Name :type String) (Position :type Integer))
  (set `self.Lyrics` Name)
  (`self.Marker`))

(event `killMusic`
  (`FMODAudioComponent.SetParameter` (`self.Audio Component`) "Volume" 0.0))

(fn `UserConstructionScript`)