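; BP_PlayerPawn is the player pawn Blueprint, handling camera and input setup for the player.
; On BeginPlay it spawns a BP_CameraActor at its Core component's transform, passes itself as the follow target, and blends the first player controller's view to it.
; It then adds the IMC_MainGame Enhanced Input mapping context.
; IA_Movement only stores its value in MovementInput, and Tick is empty.
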(event `self.ReceiveBeginPlay`
  ;[1 0.4228 0.6114] BeginPlay
  (`|ExecutionSequence`
    (:`then_0`
      (bind _returnvalue (`|SpawnActorFromClass` "/Game/Blueprints/BP_CameraActor.BP_CameraActor_C" (`SceneComponent.K2_GetComponentToWorld` (`self.Core`)) "AlwaysSpawn" "OverrideRootScale" null self null))
      (`PlayerController.SetViewTargetWithBlend` (`GameplayStatics.GetPlayerController` 0) _returnvalue 2.0 "VTBlend_Linear" 0.0 false))
    (:`then_1`
      (`EnhancedInputSubsystemInterface.AddMappingContext` (pcsubsystem `EnhancedInputLocalPlayerSubsystem` (`GameplayStatics.GetPlayerController` 0)) "/Game/Input/IMC_MainGame.IMC_MainGame" 0 (struct)))))

(event `self.ReceiveTick`
  (params (DeltaSeconds :type "Float (single-precision)")))

(event `EnhancedInput|/Game/Input/IA_Movement`
  (params (ActionValue :type "Vector2D Structure") (ElapsedSeconds :type "Float (double-precision)") (TriggeredSeconds :type "Float (double-precision)") (InputAction :type "InputAction Object Reference" :default "/Game/Input/IA_Movement.IA_Movement"))
  (:`Triggered`
    (set `self.MovementInput` ActionValue)))

(fn `UserConstructionScript`)