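; BP_Box is a puzzle box that moves one 100-unit step in its Movement direction on each beat from GM_Rizume.
; Each beat, a Visibility line trace checks the next step and, if clear, the BoxMoves timeline slides the root from its previous location.
; The game mode's ResetPuzzle event clears Movement, stops the timeline and returns the box to its start location.
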(event `self.ReceiveBeginPlay`
  (set `self.startLocation` (`SceneComponent.K2_GetComponentLocation` (`self.DefaultSceneRoot`)))
  (bind _asgm_rizume (cast `/Game/Blueprints/GM_Rizume` (`GameplayStatics.GetGameMode`)))
  (add `/Game/Blueprints/GM_Rizume.onBeat` _asgm_rizume (delegate `PersonalBeat`))
  (add `/Game/Blueprints/GM_Rizume.resetPuzzle` _asgm_rizume (delegate `Reset`)))

(event `PersonalBeat`
  (`self.boxMovement` (`self.Movement`)))

(event `Reset`
  (bind (_previouslocation_x _previouslocation_y _previouslocation_z) (`KismetMathLibrary.BreakVector` (`self.previousLocation`)))
  (bind (_movement_x _movement_y) (`KismetMathLibrary.BreakVector2D` (`self.Movement`)))
  (set `self.Movement` (0.0 0.0))
  (`SceneComponent.K2_SetWorldLocation` (`self.DefaultSceneRoot`) (`self.startLocation`) false false)
  (bind (_direction _move) (`Timeline|BoxMoves` :!via `Stop` :!label _label)
    (:`Update`
      (`SceneComponent.K2_SetWorldLocation` (`self.DefaultSceneRoot`) (`KismetMathLibrary.MakeVector` (+ (* _move 100.0 _movement_x) _previouslocation_x) (+ (* _move 100.0 _movement_y) _previouslocation_y) _previouslocation_z) false false))))

(event `boxMovement`
  (params (Direction :type "Vector2D Structure"))
  (if (!= Direction (0.0 0.0))
    (set `self.previousLocation` (`SceneComponent.K2_GetComponentLocation` (`self.DefaultSceneRoot`)))
    (bind _canmove (`self.canMove`))
    (if _canmove
      (goto _label :!via `PlayFromStart`))))

(fn `canMove`
  (returns (canMove :type Boolean))
  (bind (_movement_x _movement_y) (`KismetMathLibrary.BreakVector2D` (`self.Movement`)))
  (bind _returnvalue (`SceneComponent.K2_GetComponentLocation` (`self.DefaultSceneRoot`)))
  (bind (_outhit _returnvalue_2) (`KismetSystemLibrary.LineTraceSingle` :`Start` _returnvalue :`End` (+ _returnvalue (`KismetMathLibrary.MakeVector` (* _movement_x 100.0) (* _movement_y 100.0))) :`TraceChannel` "TraceTypeQuery1" :`DrawDebugType` "ForDuration"))
  (return (not _returnvalue_2)))

(fn `UserConstructionScript`)