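; Main menu actor that shows the WI_MainMenu widget and drives a beat-reactive camera.
; On BeginPlay it adds the menu mapping context and binds to GM_Menu's beat and intensity dispatchers.
; Once intensity rises, it changes the camera's post-process settings and rotates the camera a step on each beat.
; The interact input tells the menu widget to disappear.
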(event `self.ReceiveBeginPlay`
  (bind _returnvalue (`|GenericCreateObject` "/Game/UI/WI_MainMenu.WI_MainMenu_C"))
  (bind _output_get (set `self.menuUI` _returnvalue))
  (`UserWidget.AddToViewport` _output_get 0)
  (bind _asgm_menu (cast `/Game/Blueprints/GM_Menu` (`GameplayStatics.GetGameMode`)))
  (add `/Game/Blueprints/GM_Menu.onBeatDisp` _asgm_menu (delegate `SelfBeat`))
  (add `/Game/Blueprints/GM_Menu.intensityUp` _asgm_menu (delegate `Intensitay`))
  (`EnhancedInputSubsystemInterface.AddMappingContext` (pcsubsystem `EnhancedInputLocalPlayerSubsystem` (`GameplayStatics.GetPlayerController` 0)) "/Game/Input/IMC_Menu.IMC_Menu" 0 (struct)))

(event `Intensitay`
  (set `self.highIntensity` true)
  (set `CameraComponent.PostProcessSettings` (make `PostProcessSettings` :`ColorContrast` (`KismetMathLibrary.MakeVector4` 1.0 1.0 1.0 1.0)) (`self.Camera`)))

(event `SelfBeat`
  (if (`self.highIntensity`)
    (`self.Rotato`)))

(event `Rotato`
  (`SceneComponent.K2_AddWorldRotation` (`self.Camera`) (struct :`Roll` 7.0) false false))

(event `EnhancedInput|/Game/Input/IA_Interact`
  (params (ActionValue :type Boolean) (ElapsedSeconds :type "Float (double-precision)") (TriggeredSeconds :type "Float (double-precision)") (InputAction :type "InputAction Object Reference" :default "/Game/Input/IA_Interact.IA_Interact"))
  (:`Triggered`
    (`/Game/UI/WI_MainMenu.makeDisappear` (`self.menuUI`))))

(fn `UserConstructionScript`)