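; GM_Rizume is a game mode Blueprint that acts as the hub for music beat timing and puzzle resets.
; On BeginPlay it adds an FMOD audio component, plays TestMusic and binds to its timeline beat callback.
; Each beat stores tempo divided by 60 as TempoInterval and broadcasts OnBeat.
; A separate resetAllPuzzles event broadcasts ResetPuzzle to any listeners.
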(event `self.ReceiveBeginPlay`
  (bind _returnvalue (`AddComponent|NODE_AddFMODAudioComponent-3` :`bManualAttachment` true))
  (bind _output_get (set `self.Audio Component` _returnvalue))
  (`FMODAudioComponent.SetEvent` _output_get "/Game/FMOD/Events/Music/TestMusic.TestMusic")
  (add `FMODAudioComponent.OnTimelineBeat` _output_get (delegate `onBeatEvent`))
  (set `FMODAudioComponent.bEnableTimelineCallbacks` true _output_get)
  (`FMODAudioComponent.Play` _output_get))

(event `onBeatEvent`
  (params (Bar :type Integer) (Beat :type Integer) (Position :type Integer) (Tempo :type "Float (single-precision)") (TimeSignatureUpper :type Integer) (TimeSignatureLower :type Integer))
  (set `self.TempoInterval` (/ Tempo 60.0))
  (`self.onBeat`))

(event `resetAllPuzzles`
  (`self.resetPuzzle`))

(fn `UserConstructionScript`)