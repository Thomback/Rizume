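; BP_Grille is a puzzle gate that slides down 200 units when activated and rises back when deactivated.
; BeginPlay caches both end positions and binds Reset to the GM_Rizume game mode's puzzle-reset event.
; Two timelines, Descendre and Monter, lerp the root's Z, each stopped before the other plays, guarded by an Activated flag.
; Reset teleport-free snaps the gate to its start, clears the flag and stops both timelines.
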(event `Activate`
  (bind (_startlocation_x _startlocation_y _startlocation_z) (`KismetMathLibrary.BreakVector` (`self.startLocation`)))
  (bind (_finishlocation_x _finishlocation_y _finishlocation_z) (`KismetMathLibrary.BreakVector` (`self.finishLocation`)))
  (bind (_startlocation_x_2 _startlocation_y_2 _startlocation_z_2) (`KismetMathLibrary.BreakVector` (`self.startLocation`)))
  (bind (_finishlocation_x_2 _finishlocation_y_2 _finishlocation_z_2) (`KismetMathLibrary.BreakVector` (`self.finishLocation`)))
  (if (not (`self.activated`))
    (`|ExecutionSequence`
      (:`then_0`
        (bind (_direction _monterman) (`Timeline|monter` :!via `Stop` :!label _label)
          (:`Update`
            (`SceneComponent.K2_SetWorldLocation` (`self.DefaultSceneRoot`) (`KismetMathLibrary.MakeVector` _finishlocation_x_2 _finishlocation_y_2 (`KismetMathLibrary.Lerp` _finishlocation_z_2 _startlocation_z _monterman)) false false))))
      (:`then_1`
        (set `self.activated` true)
        (bind (_direction_2 _anim) (`Timeline|descendre` :!label _label_2)
          (:`Update`
            (`SceneComponent.K2_SetWorldLocation` (`self.DefaultSceneRoot`) (`KismetMathLibrary.MakeVector` _startlocation_x_2 _startlocation_y_2 (`KismetMathLibrary.Lerp` _startlocation_z_2 _finishlocation_z _anim)) false false)))))))

(event `self.ReceiveBeginPlay`
  (bind _output_get (set `self.startLocation` (`SceneComponent.K2_GetComponentLocation` (`self.DefaultSceneRoot`))))
  (set `self.finishLocation` (`KismetMathLibrary.MakeVector` (.x _output_get) (.y _output_get) (- (.z _output_get) 200.0)))
  (bind _asgm_rizume (cast `/Game/Blueprints/GM_Rizume` (`GameplayStatics.GetGameMode`)))
  (add `/Game/Blueprints/GM_Rizume.resetPuzzle` _asgm_rizume (delegate `Reset`)))

(event `Reset`
  (`SceneComponent.K2_SetWorldLocation` (`self.DefaultSceneRoot`) (`self.startLocation`) false false)
  (set `self.activated` false)
  (`|ExecutionSequence`
    (:`then_0`
      (goto _label_2 :!via `Stop`))
    (:`then_1`
      (goto _label :!via `Stop`))))

(event `Deactivate`
  (if (`self.activated`)
    (`|ExecutionSequence`
      (:`then_0`
        (goto _label_2 :!via `Stop`))
      (:`then_1`
        (set `self.activated` false)
        (goto _label :!via `PlayFromStart`)))))

(fn `UserConstructionScript`)