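; An actor Blueprint that reacts to the beat by setting the material on its Niagara particle system.
; The construction script creates a dynamic material instance from MaterialOff.
; On BeginPlay it casts the game mode to Menu, Rizume or Credits and binds ChangeParticle to that mode's beat event.
; Each beat assigns the same dynamic instance to the Niagara "myMat" variable; no material parameters are changed.
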(event `self.ReceiveBeginPlay`
  (bind _returnvalue (`GameplayStatics.GetGameMode`))
  (bind _asgm_menu (cast `/Game/Blueprints/GM_Menu` _returnvalue)
    (:`then`
      (add `/Game/Blueprints/GM_Menu.onBeatDisp` _asgm_menu (delegate `changeParticle`)))
    (:`CastFailed`
      (bind _asgm_rizume (cast `/Game/Blueprints/GM_Rizume` _returnvalue)
        (:`then`
          (add `/Game/Blueprints/GM_Rizume.onBeat` _asgm_rizume (delegate `changeParticle`)))
        (:`CastFailed`
          (bind _asgm_credits (cast `/Game/Blueprints/GM_Credits` _returnvalue))
          (add `/Game/Blueprints/GM_Credits.onBeat` _asgm_credits (delegate `changeParticle`)))))))

(event `changeParticle`
  (`NiagaraComponent.SetVariableMaterial` (`self.Niagara`) "myMat" (`self.Dynamic`)))

(fn `UserConstructionScript`
  (bind _returnvalue (`KismetMaterialLibrary.CreateDynamicMaterialInstance` (`self.MaterialOff`)))
  (set `self.Dynamic` _returnvalue))